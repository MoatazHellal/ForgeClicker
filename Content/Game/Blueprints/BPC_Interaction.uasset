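; BPC_Interaction is a component that detects when the mouse cursor hovers over an interactable actor and swaps the cursor to match.
; BeginPlay creates and caches the hand and default cursor widgets.
; Each Tick traces under player 0's cursor against WorldDynamic objects and checks the hit actor for BPI_Interactable, setting IsHoveringOverButton and the cursor widget.
; ButtonRef stores the hit actor in both cases, interactable or not.
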(event EventBeginPlay
  (bind _returnvalue (UserInterface|CreateWidget "/Game/Game/Widgets/WBP_Cursor_Hand.WBP_Cursor_Hand_C"))
  (Variables|Default|SetHandCursorWidgetRef _returnvalue)
  (bind _returnvalue_2 (UserInterface|CreateWidget "/Game/Game/Widgets/WBP_Cursor_Default.WBP_Cursor_Default_C"))
  (Variables|Default|SetDefaultCursorWidgetRef _returnvalue_2))

(event EventTick
  (params (DeltaSeconds :type Float%20%28single-precision%29))
  (bind _returnvalue (Game|GetPlayerController 0))
  (bind _array (Utilities|Array|MakeArray "ObjectTypeQuery2"))
  (bind _hitresult (Class|PlayerController|GetHitResultUnderCursorforObjects _returnvalue _array true))
  (bind _hitactor (Collision|BreakHitResult _hitresult))
  (if (Utilities|DoesObjectImplementInterface _hitactor "/Game/Game/Blueprints/BPI_Interactable.BPI_Interactable_C")
    (Variables|Default|SetIsHoveringOverButton true)
    (Class|PlayerController|SetMouseCursorWidget _returnvalue "Default" (Variables|Default|GetHandCursorWidgetRef))
    (Variables|Default|SetButtonRef _hitactor)
    (else
      (Variables|Default|SetIsHoveringOverButton false)
      (Class|PlayerController|SetMouseCursorWidget _returnvalue "Default" (Variables|Default|GetDefaultCursorWidgetRef))
      (Variables|Default|SetButtonRef _hitactor))))