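; Button actor that can be pressed and that grows when the size upgrade is purchased.
; Press broadcasts OnPressed, then plays a timeline that offsets the Main component downward, with an event track triggering a spatialized click sound.
; On BeginPlay it binds to the BP_GameState OnSetSize dispatcher, and each call compounds the actor's scale by a fixed multiplier, starting from unit scale.
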(event Custom|SizeUp
  ;[0.15 0.15 0.15 0.5] Bind size up upgrade purchase to set button size
  (bind _output_get (Variables|Default|SetCurrentScale (* (Variables|Default|GetCurrentScale) 1.5)))
  (Transformation|SetActorScale3D _output_get))

(event EventBeginPlay
  ;[0.15 0.15 0.15 0.5] Bind size up upgrade purchase to set button size
  (Variables|Default|SetCurrentScale "1.000000,1.000000,1.000000")
  (bind _asbp_game_state (Utilities|Casting|CastToBP_GameState (Game|GetGameState)))
  (EventDispatchers|BindEventtoOnSetSize _asbp_game_state (delegate Custom|SizeUp)))

(event EventPress
  (Default|CallOnPressed)
  ;[0.15 0.15 0.15 0.5] Pressing Animation
  (bind _press (Timeline|Timeline PlayFromStart)
    (:Update
      (Transformation|SetRelativeLocation (Variables|Default|GetMain) (Math|Vector|MakeVector 0.0 0.0 (Math|Float|Lerp 0.0 -1e+01 _press)) false false))
    (:Audio
      ;[0.15 0.15 0.15 0.5] Sfx
      (Audio|PlaySoundatLocation "/Game/Game/Audio/SoundWaves/SW_ButtonClick.SW_ButtonClick" (Transformation|GetActorLocation) "0, 0, 0" 1.0 1.0 0.0 "/Game/Game/Audio/SA_Main.SA_Main" 0 0 0))))

(fn ConstructionScript)