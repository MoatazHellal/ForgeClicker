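; BP_Cart is a cart actor that collects weapons and converts their combined price into funds when a sale happens.
; Overlapping BP_Weapon actors are stored in ObjectsInHold, and their prices accumulate in CurrentValue.
; It binds to the BP_GameState OnSold event at BeginPlay; SetFunds passes the total to Sell, resets it and deactivates held items back to their pool.
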(event Custom|SetFunds
  (bind _objectsinhold (Variables|Default|GetObjectsInHold))
  ;[0.15 0.15 0.15 0.5] Sell items and set current empty cart value to 0
  (Default|Sell (Variables|Default|GetGameStateRef) (Variables|Default|GetCurrentValue))
  (Variables|Default|SetCurrentValue 0.0)
  ;[0.15 0.15 0.15 0.5] Deactivate and return all items to pool
  (for _array_element _objectsinhold
    (Default|SetinUse _array_element false))
  (Utilities|Array|Clear _objectsinhold))

(event EventBeginPlay
  (Utilities|FlowControl|Sequence
    (:then_0
      ;[0.15 0.15 0.15 0.5] Initialize empty cart value to 0
      (Variables|Default|SetCurrentValue 0.0))
    (:then_1
      ;[0.15 0.15 0.15 0.5] Bind sell event to empty cart and get items value as funds
      (bind _asbp_game_state (Utilities|Casting|CastToBP_GameState (Game|GetGameState)))
      (bind _output_get (Variables|Default|SetGameStateRef _asbp_game_state))
      (EventDispatchers|BindEventtoOnSold _output_get (EventDispatchers|CreateEvent :!event Custom|SetFunds)))))

(event Collision|EventActorBeginOverlap
  (params (OtherActor :type Actor%20Object%20Reference))
  ;[0.15 0.15 0.15 0.5] Check if overlapped item is a valid gear item, store a reference and add its value to the cumulated current value
  (bind _returnvalue (CallFunction|IsA OtherActor "/Game/Game/Blueprints/BP_Weapon.BP_Weapon_C"))
  (if _returnvalue
    (bind _asbp_weapon (Utilities|Casting|CastToBP_Weapon OtherActor))
    (Utilities|Array|Add (Variables|Default|GetObjectsInHold) _asbp_weapon)
    (Variables|Default|SetCurrentValue (+ (Variables|/Game/Game/Blueprints/BP_Weapon.BP_Weapon_C|GetPrice _asbp_weapon) (Variables|Default|GetCurrentValue)))))

(fn ConstructionScript)