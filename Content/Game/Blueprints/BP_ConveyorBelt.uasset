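; BP_ConveyorBelt is a conveyor belt that moves pooled objects along its direction.
; Each tick it offsets every BP_PooledObject overlapping its box along the Direction component's forward vector, scaled by Speed and delta time.
; It binds to the game state's set-speed event, which raises Speed by a fixed step and updates a dynamic material's scroll parameter on the belt plane to match.
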(event Custom|SetSpeed
  ;[0.15 0.15 0.15 0.5] Bind speed purchase event to add speed
  (Variables|Default|SetSpeed (+ (Variables|Default|GetSpeed) 5e+01))
  (Rendering|Material|SetScalarParameterValue (Variables|Default|GetBeltMaterial) "SpeedY" (/ (Variables|Default|GetSpeed) 7.5e+02) :!class /Script/Engine.MaterialInstanceDynamic))

(event EventBeginPlay
  (Utilities|FlowControl|Sequence
    (:then_0
      ;[0.15 0.15 0.15 0.5] Create and store dynamic material reference to the belt
      (bind _returnvalue (Rendering|Material|CreateDynamicMaterialInstance (Variables|Default|GetPlane) 0 0 "None" :!class /Script/Engine.PrimitiveComponent))
      (Variables|Default|SetBeltMaterial _returnvalue))
    (:then_1
      ;[0.15 0.15 0.15 0.5] Bind speed purchase event to add speed
      (bind _asbp_game_state (Utilities|Casting|CastToBP_GameState (Game|GetGameState)))
      (EventDispatchers|BindEventtoOnSetSpeed _asbp_game_state (delegate Custom|SetSpeed)))))

(event EventTick
  (params (DeltaSeconds :type Float%20%28single-precision%29))
  (bind _box (Variables|Default|GetBox))
  (bind _overlappingactors (Collision|GetOverlappingActors _box "/Game/Game/Blueprints/BP_PooledObject.BP_PooledObject_C" :!class /Script/Engine.PrimitiveComponent))
  ;[0.15 0.15 0.15 0.5] Add continuous offset to push items on top of the belt forward
  (if (Utilities|Array|IsNotEmpty _overlappingactors)
    (for _array_element _overlappingactors
      (Transformation|AddActorWorldOffset _array_element (* (* DeltaSeconds (Variables|Default|GetSpeed)) (Math|Vector|GetForwardVector (Transformation|GetWorldRotation (Variables|Default|GetDirection))))))))

(fn ConstructionScript)