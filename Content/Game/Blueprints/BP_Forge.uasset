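; BP_Forge is a forge actor that plays a hammer strike when another actor begins overlapping it.
; The overlap restarts a Timeline whose Forge track lerps the Hammer component's roll to swing it.
; A Sparks event track on the same Timeline spawns Niagara sparks at the SparksLocation component and plays a sound at the actor, syncing effects to the animation.
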(event EventBeginPlay
  (|CallParentFunction) ; This node is disabled and will not be called.\nDrag off pins to build functionality.
)

(event Collision|EventActorBeginOverlap
  (params (OtherActor :type Actor%20Object%20Reference))
  (|CallParentFunction OtherActor)
  ;[0.15 0.15 0.15 0.5] Animation
  (bind _forge (Timeline|Timeline PlayFromStart)
    (:Update
      (Transformation|SetRelativeRotation (Variables|Default|GetHammer) (Math|Rotator|MakeRotator (Math|Float|Lerp 9e+01 155.0 _forge) 0.0 0.0) false false))
    (:Sparks
      ;[0.15 0.15 0.15 0.5] Vfx
      (Niagara|SpawnSystematLocation "/Game/Game/Effects/Niagara/NS_Sparks.NS_Sparks" (Transformation|GetWorldLocation (Variables|Default|GetSparksLocation)))
      ;[0.15 0.15 0.15 0.5] Sfx
      (Audio|PlaySoundatLocation "/Game/Game/Audio/SoundWaves/SW_Mine.SW_Mine" (Transformation|GetActorLocation) "0, 0, 0" 1.0 1.0 0.0 "/Game/Game/Audio/SA_Main.SA_Main" 0 0 0))))

(event EventTick
  (params (DeltaSeconds :type Float%20%28single-precision%29)))

(fn ConstructionScript
  (|CallParentFunction))