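; Mining site actor where presses of a BP_Button swing a pickaxe, producing ore every third swing.
; Ore spawns from one of three object pool components (iron, gold, diamond), defaulting to iron and switched by matching class when the GameState sets the ore in production.
; A timeline drives the pickaxe rotation and camera shake, with an event track firing spark effects and a random mining sound.
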(event Custom|Swing
  ;[0.15 0.15 0.15 0.5] Mine Ore after certain amount of swings
  (Math|Integer|IncrementInt (Variables|Default|GetSwingNumber)
    (:%20%20
      (if (>= (Variables|Default|GetSwingNumber) 3)
        (Default|SpawnfromPool (Variables|Default|GetObjectPoolInUse) (Transformation|GetWorldLocation (Variables|Default|GetOreSpawnLocation)))
        (Variables|Default|SetSwingNumber 0)
        ;[0.15 0.15 0.15 0.5] Swing animation
        (bind _swing (Timeline|Timeline PlayFromStart)
          (:Update
            (Transformation|SetRelativeRotation (Variables|Default|GetPickaxe) (Math|Rotator|Lerp(Rotator) "0.000000,0.000000,30.000000" "0.000000,0.000000,90.000000" _swing) false false)
            ;[0.15 0.15 0.15 0.5] Camera shake
            (Camera|PlayWorldCameraShake "/Game/Game/Effects/CS_MiningSiteLocalShake.CS_MiningSiteLocalShake_C" (Transformation|GetActorLocation) 0.0 5e+02))
          (:Sparks
            ;[0.15 0.15 0.15 0.5] Vfx
            (Niagara|SpawnSystematLocation "/Game/Game/Effects/Niagara/NS_Sparks.NS_Sparks" (Transformation|GetWorldLocation (Variables|Default|GetSparksLocation)))
            ;[0.15 0.15 0.15 0.5] Sfx
            (Audio|PlaySoundatLocation (.OutItem (Utilities|Array|Random (Utilities|Array|MakeArray "/Game/Game/Audio/SoundWaves/SW_Mining3.SW_Mining3" "/Game/Game/Audio/SoundWaves/SW_Mining2.SW_Mining2" "/Game/Game/Audio/SoundWaves/SW_Mining4.SW_Mining4" "/Game/Game/Audio/SoundWaves/SW_Mining5.SW_Mining5" "/Game/Game/Audio/SoundWaves/SW_Mining1.SW_Mining1"))) (Transformation|GetActorLocation) "0, 0, 0" 1.0 1.0 0.0 "/Game/Game/Audio/SA_Main.SA_Main" 0 0 0)))
        (else
          (Timeline|Timeline PlayFromStart))))))

(event Custom|SetObjectPoolInUse
  (params (OreInProduction :type BP%20Ore%20Class%20Reference))
  ;[0.15 0.15 0.15 0.5] Set the current pool in use to the selected ore in production
  (for _array_element (Utilities|Array|MakeArray (Variables|Default|GetBPC_ObjectPool_IronOre) (Variables|Default|GetBPC_ObjectPool_GoldOre) (Variables|Default|GetBPC_ObjectPool_DiamondOre))
    (if (== (Variables|/Game/Game/Blueprints/BPC_ObjectPool.BPC_ObjectPool_C|GetPooledActorClass _array_element) OreInProduction)
      (Variables|Default|SetObjectPoolInUse _array_element))))

(event EventBeginPlay
  (Utilities|FlowControl|Sequence
    (:then_0
      ;[0.15 0.15 0.15 0.5] Initiliaze pool in use to iron pool
      (Variables|Default|SetObjectPoolInUse (Variables|Default|GetBPC_ObjectPool_IronOre)))
    (:then_1
      ;[0.15 0.15 0.15 0.5] Bind event to set ore in production to the selected ore
      (bind _asbp_game_state (Utilities|Casting|CastToBP_GameState (Game|GetGameState)))
      (EventDispatchers|BindEventtoOnSetOreinProduction _asbp_game_state (EventDispatchers|CreateEvent :!event Custom|SetObjectPoolInUse)))
    (:then_2
      ;[0.15 0.15 0.15 0.5] Bind the button click to pickaxe swing
      (bind _returnvalue (Actor|GetActorOfClass "/Game/Game/Blueprints/BP_Button.BP_Button_C"))
      (EventDispatchers|BindEventtoOnPressed _returnvalue (EventDispatchers|CreateEvent :!event Custom|Swing)))))

(fn ConstructionScript)