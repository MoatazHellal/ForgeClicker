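; Base processor actor that turns overlapping ingredient actors into output items using recipes from a data table.
; A matched input is released from use, and the output's pool component (iron, gold or diamond), found through a class-keyed map, joins a FIFO queue.
; A looping timer spawns queued outputs at the spawn location, keeping the processing time of the recipe that started it until the queue empties.
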(event Custom|Process
  ;[0.15 0.15 0.15 0.5] Find corresponding recipe to the overlapped ingredient actor and set processing timer
  (Default|SpawnfromPool (Utilities|Array|Get(acopy) (Variables|Default|GetObjectPoolInUse)) (Transformation|GetWorldLocation (Variables|Default|GetOutputSpawnLocation)))
  (Utilities|Array|RemoveIndex (Variables|Default|GetObjectPoolInUse))
  (if (> (Variables|Default|GetQueuedIngredients) 0)
    (Math|Integer|DecrementInt (Variables|Default|GetQueuedIngredients))
    (else
      (Utilities|Time|ClearandInvalidateTimerbyHandle (Variables|Default|GetProcessingTimerHandle)))))

(event EventBeginPlay
  (bind _bpc_objectpool_iron (Variables|Default|GetBPC_ObjectPool_Iron))
  (bind _bpc_objectpool_diamond (Variables|Default|GetBPC_ObjectPool_Diamond))
  (bind _bpc_objectpool_gold (Variables|Default|GetBPC_ObjectPool_Gold))
  ;[0.15 0.15 0.15 0.5] Initialize map of all object pool types
  (Variables|Default|SetMap (Utilities|Map|MakeMap (Variables|/Game/Game/Blueprints/BPC_ObjectPool.BPC_ObjectPool_C|GetPooledActorClass _bpc_objectpool_iron) _bpc_objectpool_iron (Variables|/Game/Game/Blueprints/BPC_ObjectPool.BPC_ObjectPool_C|GetPooledActorClass _bpc_objectpool_gold) _bpc_objectpool_gold (Variables|/Game/Game/Blueprints/BPC_ObjectPool.BPC_ObjectPool_C|GetPooledActorClass _bpc_objectpool_diamond) _bpc_objectpool_diamond)))

(event Collision|EventActorBeginOverlap
  (params (OtherActor :type Actor%20Object%20Reference))
  ;[0.15 0.15 0.15 0.5] Find corresponding recipe to the overlapped ingredient actor and set processing timer
  (bind (_processingtime _outputitem _isrecipefound) (CallFunction|FindRecipe OtherActor))
  (if _isrecipefound
    (bind _asbp_pooled_object (Utilities|Casting|CastToBP_PooledObject OtherActor))
    (Default|SetinUse _asbp_pooled_object false)
    (Utilities|Array|Add (Variables|Default|GetObjectPoolInUse) (.Value (Utilities|Map|Find (Variables|Default|GetMap) _outputitem)))
    (if (Utilities|Time|IsTimerActivebyHandle (Variables|Default|GetProcessingTimerHandle))
      (Math|Integer|IncrementInt (Variables|Default|GetQueuedIngredients))
      (else
        (bind _returnvalue (Utilities|Time|SetTimerbyEvent (delegate Custom|Process) _processingtime true))
        (Variables|Default|SetProcessingTimerHandle _returnvalue)))))

(fn ConstructionScript)

(fn FindRecipe
  (params (InputActor :type Actor%20Object%20Reference))
  ;[0.15 0.15 0.15 0.5] Search data table for a row with same input as the param and return corresponding data
  (bind _outrownames (DataTable|GetDataTableRowNames (Variables|Default|GetRecipeTable)))
  (for _array_element _outrownames
    (bind _returnvalue (Utilities|GetDataTableRow (Variables|Default|GetRecipeTable) _array_element)
      (:then
        (if (== (.InputItem (Utilities|Struct|BreakStruct_Recipe _returnvalue)) (Utilities|GetClass InputActor))
          (return (.ProcessingTime (Utilities|Struct|BreakStruct_Recipe _returnvalue)) (.OutputItem (Utilities|Struct|BreakStruct_Recipe _returnvalue)) true)))))
  (return 0.0 0 false))