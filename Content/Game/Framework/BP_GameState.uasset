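; Game state for an ore production economy game, holding the player's funds and hosting the HUD and background music.
; On BeginPlay it creates the HUD and binds its ore, upgrade and sell buttons.
; Unlocks and upgrades deduct funds through a clamped Buy, while event dispatchers broadcast ore selection, sales and speed or size upgrades.
; Selling only broadcasts and plays a sound, with a separate Sell function adding funds.
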(event Custom|SetOreInProduction
  (params (OreType :type BP%20Ore%20Class%20Reference))
  ;[0.15 0.15 0.15 0.5] Bind ore production widget's buttons
  (Default|CallOnSetOreinProduction OreType))

(event Custom|SetFunds
  ;[0.15 0.15 0.15 0.5] Bind sell event
  (Default|CallOnSold)
  (Audio|PlaySound2D "/Game/Game/Audio/SoundWaves/SW_Transaction.SW_Transaction" 1.0 1.0 0.0 0 0))

(event Custom|Purchase
  (params (Price :type Float%20%28double-precision%29))
  ;[0.15 0.15 0.15 0.5] Bind ore production widget's buttons
  (CallFunction|Buy Price)
  (Audio|PlaySound2D "/Game/Game/Audio/SoundWaves/SW_Transaction.SW_Transaction" 1.0 1.0 0.0 0 0))

(event Custom|PurchaseUpgrade
  (params (Price :type Float%20%28double-precision%29) (Type :type Enum_UpgradeType%20Enum :default "NewEnumerator0"))
  ;[0.15 0.15 0.15 0.5] Bind upgrade widget's buttons
  (CallFunction|Purchase Price)
  (switch Utilities|FlowControl|Switch|SwitchonEnum_UpgradeType Type
    (:NewEnumerator0
      (Default|CallOnSetSpeed))
    (:NewEnumerator1
      (Default|CallOnSetSize))))

(event EventBeginPlay
  (Variables|Default|SetCurrentFunds 0.0)
  (bind _returnvalue (UserInterface|CreateWidget "/Game/Game/Widgets/WBP_HUD.WBP_HUD_C"))
  (bind _output_get (Variables|Default|SetHUDWidget _returnvalue))
  (UserInterface|Viewport|AddtoViewport _output_get 0)
  (Utilities|FlowControl|Sequence
    (:then_0
      ;[0.15 0.15 0.15 0.5] Initialize background music
      (Audio|PlaySound2D "/Game/Game/Audio/SoundWaves/SW_BGM.SW_BGM" 1.0 1.0 0.0 0 0))
    (:then_1
      ;[0.15 0.15 0.15 0.5] Bind ore production widget's buttons
      (for _array_element (Variables|/Game/Game/Widgets/WBP_HUD.WBP_HUD_C|GetOre%20Buttons (Variables|Default|GetHUDWidget))
        (EventDispatchers|BindEventtoOnOreSelected _array_element (delegate Custom|SetOreInProduction))
        (EventDispatchers|BindEventtoOnOreUnlocked _array_element (delegate Custom|Purchase))))
    (:then_2
      ;[0.15 0.15 0.15 0.5] Bind sell event
      (EventDispatchers|BindEventtoOnSell (Variables|Default|GetHUDWidget) (delegate Custom|SetFunds)))
    (:then_3
      ;[0.15 0.15 0.15 0.5] Bind upgrade widget's buttons
      (for _array_element_2 (Variables|/Game/Game/Widgets/WBP_HUD.WBP_HUD_C|GetUgrade%20Buttons (Variables|Default|GetHUDWidget))
        (EventDispatchers|BindEventtoOnUpgradePurchased _array_element_2 (delegate Custom|PurchaseUpgrade))))))

(fn ConstructionScript)

(fn Sell
  (params (Amount :type Float%20%28double-precision%29))
  (Variables|Default|SetCurrentFunds (+ Amount (Variables|Default|GetCurrentFunds))))

(fn Buy
  (params (Amount :type Float%20%28double-precision%29))
  (Variables|Default|SetCurrentFunds (Math|Float|Clamp(Float) (- (Variables|Default|GetCurrentFunds) Amount) 0.0 999999.0)))